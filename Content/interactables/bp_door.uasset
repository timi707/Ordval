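; An interactable door actor that swings open and closed when the player interacts with it.
; Interact plays a locked-handle sound if Locked, otherwise it plays a creak and runs the OpenDoor or CloseDoor timeline based on the Closed flag, driving the door mesh's relative yaw.
; A Moving flag ignores input until the swing finishes.
; Hover returns a type and the door's Name for interaction feedback.
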(event EventBeginPlay)

(event Collision|EventActorBeginOverlap
  (params (OtherActor :type Actor%20Object%20Reference)))

(event EventTick
  (params (DeltaSeconds :type Float%20%28single-precision%29)))

(event EventInteract
  (bind _returnvalue (Transformation|GetActorLocation))
  (if (Variables|Default|Getlocked?)
    (Audio|PlaySoundatLocation "/Game/ProSoundCollection_v1_3/Doors/Cues/door_lock_handle_locked_01_Cue.door_lock_handle_locked_01_Cue" _returnvalue "0, 0, 0" 1.0 1.0 0.0 0 0 0 0)
    (elif (not (Variables|Default|Getmoving?))
      (Variables|Default|Setmoving? true)
      (if (Variables|Default|Getclosed?)
        (Audio|PlaySoundatLocation "/Game/ProSoundCollection_v1_3/Doors/Cues/door_A_creak_02_Cue.door_A_creak_02_Cue" _returnvalue "0, 0, 0" 1.0 1.0 0.0 0 0 0 0)
        (bind _newtrack_0 (Timeline|open%20door PlayFromStart)
          (:Update
            (Transformation|SetRelativeRotation (Variables|Default|GetdoorMesh) (Math|Rotator|MakeRotator 0.0 0.0 _newtrack_0) false false))
          (:Finished
            (Variables|Default|Setclosed? false)
            (Variables|Default|Setmoving? false :!label _label)))
        (else
          (Audio|PlaySoundatLocation "/Game/ProSoundCollection_v1_3/Doors/Cues/door_A_creak_03_Cue.door_A_creak_03_Cue" _returnvalue "0, 0, 0" 1.0 1.0 0.0 0 0 0 0)
          (bind _newtrack_0_2 (Timeline|close%20door PlayFromStart)
            (:Update
              (Transformation|SetRelativeRotation (Variables|Default|GetdoorMesh) (Math|Rotator|MakeRotator 0.0 0.0 _newtrack_0_2) false false))
            (:Finished
              (Variables|Default|Setclosed? true)
              (goto _label))))))))

(fn ConstructionScript)

(fn Hover
  (return "NewEnumerator0" (Variables|Default|Getname)))