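; Interactable dummy actor that takes damage from the player and shows up as "Dummy" on hover.
; Its Damage event subtracts the base damage from Health only when player-caused, with no death handling.
; GetType supplies its surface type and sound, while Hover supplies the interaction type and name.
; A play-sound node at the actor's location is left disconnected, so it never runs.
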(event EventBeginPlay)

(event Collision|EventActorBeginOverlap
  (params (OtherActor :type Actor%20Object%20Reference)))

(event EventTick
  (params (DeltaSeconds :type Float%20%28single-precision%29)))

(event EventDamage
  (params (playerCaused? :type Boolean) (element :type Integer) (baseDamage :type Float%20%28double-precision%29) (type :type Integer))
  (if playerCaused?
    (Variables|Default|Sethealth (- (Variables|Default|Gethealth) baseDamage))))

(fn ConstructionScript)

(fn GetType
  (return (Variables|Default|GetSurface%20Type) (Variables|Default|GetSound)))

(fn Hover
  (return "NewEnumerator8" "Dummy"))