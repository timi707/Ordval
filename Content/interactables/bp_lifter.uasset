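; BP_Lifter is an interactable lift volume that floats the player upward while they are inside its capsule.
; Overlapping the capsule zeroes the player's gravity scale and stores the reference; leaving resets gravity to normal.
; While the player is inside, Tick calls LaunchCharacter with a small upward velocity that adds to their current velocity.
; The construction script sets the capsule half-height from a Height variable.
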(event OnComponentBeginOverlap(Capsule)
  (params (OverlappedComponent :type Primitive%20Component%20Object%20Reference) (OtherActor :type Actor%20Object%20Reference) (OtherComp :type Primitive%20Component%20Object%20Reference) (OtherBodyIndex :type Integer) (bFromSweep :type Boolean) (SweepResult :type Hit%20Result%20Structure%20%28by%20ref%29))
  (bind _asbp_player (Utilities|Casting|CastToBP_Player OtherActor))
  (Variables|/Script/Engine.CharacterMovementComponent|SetGravityScale (Variables|/Script/Engine.Character|GetCharacterMovement _asbp_player) 0.0)
  (Variables|Default|SetAs%20BP%20Player _asbp_player)
  (Variables|Default|SetplayerIn true))

(event OnComponentEndOverlap(Capsule)
  (params (OverlappedComponent :type Primitive%20Component%20Object%20Reference) (OtherActor :type Actor%20Object%20Reference) (OtherComp :type Primitive%20Component%20Object%20Reference) (OtherBodyIndex :type Integer))
  (bind _asbp_player (Utilities|Casting|CastToBP_Player OtherActor))
  (Variables|/Script/Engine.CharacterMovementComponent|SetGravityScale (Variables|/Script/Engine.Character|GetCharacterMovement _asbp_player) 1.0)
  (Variables|Default|SetplayerIn false))

(event EventBeginPlay)

(event Collision|EventActorBeginOverlap
  (params (OtherActor :type Actor%20Object%20Reference)))

(event EventTick
  (params (DeltaSeconds :type Float%20%28single-precision%29))
  (if (Variables|Default|GetplayerIn)
    (Character|LaunchCharacter (Variables|Default|GetAs%20BP%20Player) "0.000000,0.000000,1.000000" false false)))

(fn ConstructionScript
  (Components|Capsule|SetCapsuleHalfHeight (Variables|Default|GetCapsule) (Variables|Default|Getheight) true))